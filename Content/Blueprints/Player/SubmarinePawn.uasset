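; Player submarine pawn for a side-view Paper2D game, with motor-gated movement, a mouse-aimed torch and health.
; Releasing ToggleMotor flips the motor state; switching it on starts Wwise engine audio and freezes the flipbook on a set frame.
; Each tick syncs torch visibility to its flag and aims it at the deprojected cursor on the XZ plane.
; Damage reduces health, and at zero or below plays the animation on Alarm widgets.
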(event EventBeginPlay
  (Components|Timeline|SetNewTime (Variables|Default|GetPaperFlipbook) 1.0))

(event Collision|EventActorBeginOverlap
  (params (OtherActor :type Actor%20Object%20Reference)))

(event Game|Damage|EventAnyDamage
  (params (Damage :type Float%20%28single-precision%29) (DamageType :type Damage%20Type%20Object%20Reference) (InstigatedBy :type Controller%20Object%20Reference) (DamageCauser :type Actor%20Object%20Reference))
  (Variables|Default|SetHealth (- (Variables|Default|GetHealth) Damage))
  (if (<= (Variables|Default|GetHealth) 0.0)
    (bind _foundwidgets (Widget|GetAllWidgetsOfClass "/Game/UI/Alarm.Alarm_C" true))
    (for _array_element _foundwidgets
      (UserInterface|Animation|PlayAnimation _array_element (Variables|/Game/UI/Alarm.Alarm_C|GetAlarmOn _array_element) 0.0 0 "Forward" 1.0))
    (Development|PrintString (Utilities|String|ToString(Float) (Variables|Default|GetHealth)) true false "(R=0.234774,G=1.000000,B=0.000000,A=1.000000)" 0.0)))

(event EventTick
  (params (DeltaSeconds :type Float%20%28single-precision%29)))

(event EventTick
  (params (DeltaSeconds :type Float%20%28single-precision%29))
  (Rendering|SetVisibility (Variables|Default|GetTorch) (Variables|Default|GetIsTorchEnabled) true)
  (CallFunction|UpdateTorchMovement))

(event Input|ActionEvents|InputActionToggleMotor
  (params (Key :type Key%20Structure))
  (bind _paperflipbook (Variables|Default|GetPaperFlipbook))
  (:Released
    (bind _output_get (Variables|Default|SetIsMotorEnabled (not (Variables|Default|GetIsMotorEnabled))))
    (if _output_get
      (Class|AkGameplayStatics|PostEvent "/Game/Sounds/Events/Engine.Engine" (Game|Player|GetPlayerPawn 0))
      (Class|AkGameplayStatics|SetState "Engine" "StartEngine")
      (if (Variables|Default|GetIsMotorEnabled)
        (Class|PaperFlipbookComponent|SetPlaybackPositioninFrames _paperflipbook 2 false)
        (else
          (Class|PaperFlipbookComponent|SetPlaybackPositioninFrames (Variables|Default|GetPaperFlipbook) 1 false)))
      (Components|Timeline|SetPlayRate _paperflipbook 0.0))))

(event Input|AxisEvents|InputAxisMoveRightLeft
  (params (AxisValue :type Float%20%28single-precision%29))
  (if (Variables|Default|GetIsMotorEnabled)
    (Pawn|Input|AddMovementInput (.X (Math|Rotator|BreakRotIntoAxes (Pawn|GetControlRotation :!class /Script/Engine.Pawn))) AxisValue false)))

(event Input|AxisEvents|InputAxisMoveRightLeft
  (params (AxisValue :type Float%20%28single-precision%29)))

(event Input|AxisEvents|InputAxisMoveUpDown
  (params (AxisValue :type Float%20%28single-precision%29))
  (if (Variables|Default|GetIsMotorEnabled)
    (Pawn|Input|AddMovementInput (.Z (Math|Rotator|BreakRotIntoAxes (Pawn|GetControlRotation :!class /Script/Engine.Pawn))) AxisValue false)))

(fn ConstructionScript)

(fn UpdateTorchMovement
  (bind _returnvalue (Game|GetPlayerController 0))
  (bind _torch (Variables|Default|GetTorch))
  (bind (_worldlocation _worlddirection) (Game|Player|ConvertMouseLocationToWorldSpace _returnvalue))
  (bind (_x _y _z) (Math|Vector|BreakVector _worldlocation))
  (bind (_x_2 _y_2 _z_2) (Math|Vector|BreakVector _worlddirection))
  (bind _returnvalue_2 (Math|Vector2D|MakeVector2D _x_2 _z_2))
  (bind _returnvalue_3 (Math|Vector2D|MakeVector2D _x _z))
  (bind _returnvalue_4 (* _returnvalue_2 1e+03))
  (bind _returnvalue_5 (+ _returnvalue_3 _returnvalue_4))
  (bind (_x_3 _y_3) (Math|Vector2D|BreakVector2D _returnvalue_5))
  (if (Variables|Default|GetIsTorchEnabled)
    (Transformation|SetRelativeRotation _torch (Math|Rotator|FindLookatRotation (Transformation|GetWorldLocation _torch) (Math|Vector|MakeVector _x_3 5e+01 _y_3)) false false)))